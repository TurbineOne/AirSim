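; Vent_02 is a configurable vent prop Blueprint from an ArchVis asset pack, with no active gameplay logic.
; Its construction script creates a dynamic instance of the M_AVP1_FIX_Master material on slot 0 of the static mesh.
; The Blueprint's variables feed that instance's base color tint, base color, mask and normal textures, and emissive color and power, so the look is set at construction.
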(event EventBeginPlay)

(event Collision|EventActorBeginOverlap
  (params (OtherActor :type Actor%20Object%20Reference)))

(event EventTick
  (params (DeltaSeconds :type Float%20%28single-precision%29)))

(fn ConstructionScript
  (bind _returnvalue (Rendering|Material|CreateDynamicMaterialInstance (Variables|Setup|GetStatic%20Mesh) 0 "/Game/ArchVisPolishPack01/Materials/M_AVP1_FIX_Master.M_AVP1_FIX_Master" :!class /Script/Engine.PrimitiveComponent))
  (bind _output_get (Variables|Setup|SetMyDynMatInst _returnvalue))
  (Rendering|Material|SetVectorParameterValue _output_get "Base Color Tint" (Variables|Setup|GetColor%20Tint) :!class /Script/Engine.MaterialInstanceDynamic) ; Color Tint
  (Rendering|Material|SetTextureParameterValue _output_get "Base Color" (Variables|Setup|GetBase%20Color%20Texture)) ; Base Color Texture
  (Rendering|Material|SetTextureParameterValue _output_get "Masks" (Variables|Setup|GetMask%20Texture)) ; Masks Texture
  (Rendering|Material|SetTextureParameterValue _output_get "Normal" (Variables|Setup|GetNormal%20Texture)) ; Normal Texture
  (Rendering|Material|SetVectorParameterValue _output_get "Emissive Color" (Variables|Setup|GetEmissive%20Color) :!class /Script/Engine.MaterialInstanceDynamic) ; Emissive Color/Power
  (Rendering|Material|SetScalarParameterValue _output_get "Emissive Power" (Variables|Setup|GetEmissive%20Power) :!class /Script/Engine.MaterialInstanceDynamic))