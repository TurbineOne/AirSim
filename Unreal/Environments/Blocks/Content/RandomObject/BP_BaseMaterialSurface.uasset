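; BP_BaseMaterialSurface is a surface actor whose static mesh keeps switching to random base textures.
; BeginPlay creates a dynamic instance of CrystalineMaterial on the mesh's first material slot.
; UpdateMaterial sets its "Base Color" texture to a random WeirdBackgroundList entry and applies it.
; MaterialTimer repeats that update and sets the timer again, so each swap gets a new short random interval.
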(event Custom|MaterialTimer
  (CallFunction|UpdateMaterial (Variables|Default|GetStaticMesh) (stale EventBeginPlay _returnvalue) (stale EventBeginPlay _returnvalue))
  (Utilities|Time|SetTimerbyEvent (delegate Custom|MaterialTimer) (Math|Random|RandomFloatinRange 0.0 1.5) true))

(event EventBeginPlay
  (bind _staticmesh (Variables|Default|GetStaticMesh))
  (bind _returnvalue (Rendering|Material|CreateDynamicMaterialInstance _staticmesh 0 "/Game/MyMaterials/CrystalineMaterial.CrystalineMaterial" "None" :!class /Script/Engine.PrimitiveComponent))
  (CallFunction|UpdateMaterial _staticmesh _returnvalue _returnvalue)
  (Utilities|Time|SetTimerbyEvent (delegate Custom|MaterialTimer) (Math|Random|RandomFloatinRange 0.0 1.5) true))

(fn ConstructionScript)

(fn DoonSecond
  (params (Target :type Boolean)))

(fn UpdateMaterial
  (params (self2 :type Primitive%20Component%20Object%20Reference) (Material :type Material%20Interface%20Object%20Reference) (self3 :type Material%20Instance%20Dynamic%20Object%20Reference))
  (Rendering|Material|SetTextureParameterValue self3 "Base Color" (Utilities|Array|Get(acopy) (Variables|Default|GetWeird%20Background%20List) (Math|Random|RandomIntegerinRange 0 (- (Utilities|Array|Length (Variables|Default|GetWeird%20Background%20List)) 1))))
  (Rendering|Material|SetMaterial self2 0 Material))