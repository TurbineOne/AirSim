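; BP_ItemSpawner is an actor that fills the space around itself with random items when play begins.
; On BeginPlay, SpawnObject spawns a random count of well over a thousand actors, each picked at random from the ItemsToSpawn array.
; Each gets a random rotation and sits in a random direction at a fixed distance, forming a spherical shell, with spawning forced despite collisions.
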(event EventBeginPlay
  (CallFunction|SpawnObject))

(fn ConstructionScript)

(fn SpawnObject
  (for _index (range 0 (Math|Random|RandomIntegerinRange 1300 2000))
    (Game|SpawnActorfromClass (Utilities|Array|Get(acopy) (Variables|Default|GetItems_To_Spawn) (Math|Random|RandomIntegerinRange 0 (- (Utilities|Array|Length (Variables|Default|GetItems_To_Spawn)) 1))) (Math|Transform|MakeTransform (+ (Transformation|GetActorLocation) (* (Math|Random|RandomUnitVector) "1500.000000,1500.000000,1500.000000")) (Math|Conversions|RotationFromXVector (Math|Random|RandomUnitVector))) "AdjustIfPossibleButAlwaysSpawn" 0 0)))